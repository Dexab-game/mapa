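; BP_pirat is an enemy pirate character that chases the player and attacks in melee.
; Tick halts its movement until PawnSensing sees a pawn, which latches a seen flag and starts an AIMoveTo toward the player.
; On arrival it plays a Viking attack montage and damages player-tagged actors in a sphere overlap at an arrow component.
; Damage taken lowers and prints health, destroying the actor at zero.
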(event `self.ReceiveTick`
  (params (DeltaSeconds :type "Float (single-precision)"))
  (if (not (`self.iSseePlayer?`))
    (`MovementComponent.StopMovementImmediately` (`self.CharacterMovement`))))

(event `self.PawnSensing.OnSeePawn`
  (params (Pawn :type "Pawn Object Reference"))
  (set `self.iSseePlayer?` true)
  (`self.followplayer`))

(event `followplayer`
  (set `self.canAttack?` true)
  (if (`self.iSseePlayer?`)
    (`|AIMoveTo` self (0.0 0.0 0.0) (`GameplayStatics.GetPlayerCharacter` 0) 50.0
      (:`OnSuccess`
        (if (`self.canAttack?`)
          (set `self.canAttack?` false)
          (bind _returnvalue (`self.PlayAnimMontage` "/Game/Viking/Animations/Anim_Viking_attack1_Montage.Anim_Viking_attack1_Montage"))
          (bind _outactors (`KismetSystemLibrary.SphereOverlapActors` (`SceneComponent.K2_GetComponentLocation` (`self.Arrow1`)) 100.0 (`self.Object Types`)))
          (for _array_element _outactors
            (if (`self.ActorHasTag` _array_element "player")
              (`GameplayStatics.ApplyDamage` _array_element 10.0)))
          (`KismetSystemLibrary.Delay` _returnvalue)
          (set `self.canAttack?` false))))
    (else
      (set `self.iSseePlayer?` false))))

(event `self.ReceiveAnyDamage`
  (params (Damage :type "Float (single-precision)") (DamageType :type "DamageType Object Reference") (InstigatedBy :type "Controller Object Reference") (DamageCauser :type "Actor Object Reference"))
  (set `self.health` (- (`self.health`) Damage))
  (`KismetSystemLibrary.PrintString` (`KismetStringLibrary.Conv_DoubleToString` (`self.health`)))
  (if (<= (`self.health`) 0.0)
    (`self.K2_DestroyActor`)))

(fn `UserConstructionScript`)